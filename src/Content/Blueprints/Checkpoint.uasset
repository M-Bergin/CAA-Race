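; Checkpoint actor for BP_TeslaVehicle that records respawn points and penalizes wrong-way driving.
; On actor overlap, a dot product of vehicle velocity and the Arrow's forward vector checks travel direction.
; Forward passes set the respawn location ahead of the Arrow, its direction, and increment the cleared-checkpoint count.
; Non-forward entry, or non-forward exit from the Trigger, sets the vehicle's respawn flag; trigger-disable and CheckpointCleared calls are unconnected.
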(event OnComponentEndOverlap(Trigger)
  (params (OverlappedComponent :type Primitive%20Component%20Object%20Reference) (OtherActor :type Actor%20Object%20Reference) (OtherComp :type Primitive%20Component%20Object%20Reference) (OtherBodyIndex :type Integer))
  (bind _asbp_tesla_vehicle (Utilities|Casting|CastToBP_TeslaVehicle OtherActor))
  (if (not (> (Math|Vector|DotProduct (Transformation|GetVelocity _asbp_tesla_vehicle) (Math|Rotator|GetRotationXVector (Transformation|GetWorldRotation (Variables|Default|GetArrow)))) 0.0))
    (Variables|/Game/Tesla_import/BP_TeslaVehicle.BP_TeslaVehicle_C|SetRespawnBool _asbp_tesla_vehicle true)))

(event Collision|EventActorBeginOverlap
  (params (OtherActor :type Actor%20Object%20Reference))
  (bind _arrow (Variables|Default|GetArrow))
  (bind _returnvalue (Transformation|GetWorldRotation _arrow))
  (bind _returnvalue_2 (Math|Rotator|GetRotationXVector _returnvalue))
  ;[1 1 1] Checkpoint system
  (bind _asbp_tesla_vehicle (Utilities|Casting|CastToBP_TeslaVehicle OtherActor))
  (if (> (Math|Vector|DotProduct (Transformation|GetVelocity _asbp_tesla_vehicle) _returnvalue_2) 0.0)
    (Variables|/Game/Tesla_import/BP_TeslaVehicle.BP_TeslaVehicle_C|SetRespawnLocation _asbp_tesla_vehicle (+ (Transformation|GetWorldLocation (Variables|Default|GetArrow)) (* _returnvalue_2 5e+02)))
    (Variables|/Game/Tesla_import/BP_TeslaVehicle.BP_TeslaVehicle_C|SetRespawnDirection _asbp_tesla_vehicle _returnvalue_2)
    (Variables|/Game/Tesla_import/BP_TeslaVehicle.BP_TeslaVehicle_C|SetCheckpointsClearedNum _asbp_tesla_vehicle (+ (Variables|/Game/Tesla_import/BP_TeslaVehicle.BP_TeslaVehicle_C|GetCheckpointsClearedNum _asbp_tesla_vehicle) 1))
    (else
      (Variables|/Game/Tesla_import/BP_TeslaVehicle.BP_TeslaVehicle_C|SetRespawnBool _asbp_tesla_vehicle true))))

(fn ConstructionScript)