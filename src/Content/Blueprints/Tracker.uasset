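; Tracker actor that numbers a list of checkpoints and listens for them being cleared, apparently as groundwork for lap tracking.
; On BeginPlay it gives each checkpoint a one-based number, stores the total, and binds every checkpoint's cleared event from a nested loop that repeats per checkpoint.
; The cleared event passes the next checkpoint to LapCheck, which only stores it locally, so no lap logic is implemented yet.
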(event Custom|Checkpoint_Cleared
  (params (NextCheckpoint :type Integer))
  (CallFunction|LapCheck NextCheckpoint))

(event EventBeginPlay
  (for (_array_element _array_index) (Variables|Checkpoints|GetCheckpoints)
    (Variables|/Game/Blueprints/Checkpoint.Checkpoint_C|SetCheckpointNumber _array_element (+ _array_index 1))
    (Variables|Default|SetTotalCheckpoints (Utilities|Array|Length (Variables|Checkpoints|GetCheckpoints)))
    (for _array_element_2 (Variables|Checkpoints|GetCheckpoints)
      (EventDispatchers|AssignCheckpointCleared _array_element_2 (delegate Custom|Checkpoint_Cleared)))))

(fn ConstructionScript)

(fn LapCheck
  (params (Checkpoint :type Integer))
  (LocalVariables|SetLocalCheckpoint Checkpoint))