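; Player-driven Tesla vehicle pawn for a checkpoint race with quiz questions and an energy budget.
; Energy scales throttle, drains with input and idling, drops on respawn and rises on correct answers.
; Tick polls GameInstance flags for race start and end, updates engine audio and HUD, and triggers respawns.
; It creates the player's widgets and runs countdowns and game-over screen; activity and driver-change timer startup is disconnected.
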(event Custom|RespawnEvent_Event
  (bind _mesh (Variables|Character|GetMesh))
  ;[1 1 1] Respawn
  (Transformation|SetActorLocation (+ (Variables|Default|GetRespawnLocation) (Variables|Default|GetRespawn_shift)) false true)
  (Transformation|SetActorRotation (Math|Conversions|RotationFromXVector (Variables|Default|GetRespawnDirection)) true)
  (Physics|SetPhysicsLinearVelocity _mesh "0, 0, 0" false "None")
  (Class|PrimitiveComponent|SetPhysicsAngularVelocityinRadians _mesh "0, 0, 0" false "None")
  (Variables|Default|SetEnergy (- (Variables|Default|GetEnergy) (Variables|Default|GetEnergyRespawnPenalty))))

(event Custom|SubtractSec_Event
  ;[1 1 1] Subtract second event
  (Variables|Default|SetGameTimer (- (Variables|Default|GetGameTimer) (Math|Timespan|MakeTimespan 0 0 0 1))))

(event Custom|Activity
  (bind _activitychangeui_ref (Variables|Default|GetActivityChangeUI_ref))
  (bind _activitychangeui_ref_2 (Variables|Default|GetActivityChangeUI_ref))
  ;[1 1 1] Activity timer
  (Math|Integer|IncrementInt (Variables|Default|GetActivity_index)
    (:%20%20
      (CallFunction|QuestionCheckEvent)
      (Audio|PlaySound2D "/Game/UI_test/zapsplat_bell_med_small_school_hand_ring_med_001_39308.zapsplat_bell_med_small_school_hand_ring_med_001_39308" 1.0 1.0 0.0 0 0)
      (UserInterface|Animation|PlayAnimation _activitychangeui_ref (Variables|/Game/UI_test/ActivityChangeUI.ActivityChangeUI_C|GetFadeIn _activitychangeui_ref) 0.0 1 "Forward" 1.0 false)
      (Utilities|FlowControl|Delay (Variables|Default|GetActivity_change_window))
      (UserInterface|Animation|PlayAnimation _activitychangeui_ref_2 (Variables|/Game/UI_test/ActivityChangeUI.ActivityChangeUI_C|GetFadeOut _activitychangeui_ref_2) 0.0 1 "Forward" 1.0 false)
      (if (> (Utilities|Array|Length (Variables|Default|GetActivity_times)) (Variables|Default|GetActivity_index))
        (Utilities|Time|SetTimerbyEvent (delegate Custom|Activity) (Utilities|Array|Get(acopy) (Variables|Default|GetActivity_times) (Variables|Default|GetActivity_index)))))))

(event Custom|Question_check_Event
  ;[1 1 1] Question event
  (if (== (Math|Integer|%(Integer) (Variables|Default|GetActivity_index) 2) 1)
    (if (== (Variables|Default|GetAnswer_num) (Utilities|Array|Get(acopy) (Variables|Default|GetQuestion_answers) (- (Variables|Default|GetActivity_index) 1)))
      (Variables|Default|SetAnswer_num 3)
      (Variables|Default|SetEnergyInput true)
      (Variables|Default|SetEnergyAdded (Variables|Default|GetQuestion_energy))
      (else
        (Variables|Default|SetAnswer_num 4)))))

(event Custom|EnergyTimeoutEvent
  (Variables|Default|SetEnergyTimeout false))

(event Custom|DriverChangeEvent
  (bind _driverchangeui_ref (Variables|Default|GetDriverChangeUI_ref))
  (bind _driverchangeui_ref_2 (Variables|Default|GetDriverChangeUI_ref))
  ;[1 1 1] DriverChangeEvent
  (UserInterface|Animation|PlayAnimation _driverchangeui_ref (Variables|/Game/UI_test/DriverChangeUI.DriverChangeUI_C|GetFadeIn _driverchangeui_ref) 0.0 1 "Forward" 1.0 false)
  (Game|SetGamePaused true)
  (Utilities|FlowControl|Delay (Variables|Default|GetDriverChangeWindow))
  (UserInterface|Animation|PlayAnimation _driverchangeui_ref_2 (Variables|/Game/UI_test/DriverChangeUI.DriverChangeUI_C|GetFadeOut _driverchangeui_ref_2) 0.0 1 "Forward" 1.0 false)
  (Game|SetGamePaused false))

(event Custom|GameOverGen_Event
  (bind _mesh (Variables|Character|GetMesh))
  (bind _as_my_game_instance (Variables|Default|GetAs%20My%20Game%20Instance))
  (bind _startcountdownuiref (Variables|Default|GetStartCountdownUIRef))
  ;[1 1 1] Game over handling
  (Variables|/Game/UI_test/StartCountdownUI.StartCountdownUI_C|SetReady_text _startcountdownuiref "3")
  (Variables|/Game/UI_test/StartCountdownUI.StartCountdownUI_C|SetStart_end_text _startcountdownuiref "Race Ends In")
  (Variables|/Game/UI_test/StartCountdownUI.StartCountdownUI_C|SetMenu%20visiblity _startcountdownuiref "Visible")
  (Utilities|FlowControl|Delay 1.0)
  (Variables|/Game/UI_test/StartCountdownUI.StartCountdownUI_C|SetReady_text _startcountdownuiref "2")
  (Utilities|FlowControl|Delay 1.0)
  (Variables|/Game/UI_test/StartCountdownUI.StartCountdownUI_C|SetReady_text _startcountdownuiref "1")
  (Utilities|FlowControl|Delay 1.0)
  (Variables|/Game/UI_test/StartCountdownUI.StartCountdownUI_C|SetMenu%20visiblity _startcountdownuiref "Hidden")
  (if (Variables|Default|GetEndScreenGen)
    (Variables|Default|SetPowerBool false)
    (Widget|RemovefromParent (Variables|Default|GetWidget_ref))
    (bind _asplayer_controller (Utilities|Casting|CastToPlayerController (Pawn|GetController)))
    (bind _returnvalue (UserInterface|CreateWidget "/Game/UI_test/GameOver.GameOver_C" _asplayer_controller))
    (bind _output_get (Variables|Default|SetGameOver_widgetref _returnvalue))
    (UserInterface|Viewport|AddtoPlayerScreen _output_get)
    (Variables|/Game/UI_test/GameOver.GameOver_C|SetCheckpointsComplete (Variables|Default|GetGameOver_widgetref) (Variables|Default|GetCheckpointsClearedNum))
    (Class|WheeledVehicleMovementComponent|SetThrottleInput (Variables|Default|GetVehicleMovement) 0.0)
    (Physics|SetPhysicsLinearVelocity _mesh "0, 0, 0" false "None")
    (Class|PrimitiveComponent|SetPhysicsAngularVelocityinRadians _mesh "0, 0, 0" false "None")
    (bind _asplayer_controller_2 (Utilities|Casting|CastToPlayerController (Pawn|GetController)))
    (Variables|/Script/Engine.PlayerController|SetbShowMouseCursor _asplayer_controller_2 true)
    (Game|SetGamePaused true)
    (Variables|/Game/MainMenu/MyGameInstance.MyGameInstance_C|SetGameOverBool _as_my_game_instance false)
    (Variables|/Game/MainMenu/MyGameInstance.MyGameInstance_C|SetQuestionsDone _as_my_game_instance false)
    (Variables|/Game/MainMenu/MyGameInstance.MyGameInstance_C|SetGameStartBool _as_my_game_instance false)))

(event Custom|StartRace_Event
  (bind _startcountdownuiref (Variables|Default|GetStartCountdownUIRef))
  (Variables|/Game/UI_test/StartCountdownUI.StartCountdownUI_C|SetStart_visiblity _startcountdownuiref "Hidden")
  (Variables|/Game/UI_test/StartCountdownUI.StartCountdownUI_C|SetReady_text _startcountdownuiref "3")
  (Variables|/Game/UI_test/StartCountdownUI.StartCountdownUI_C|SetStart_end_text _startcountdownuiref "Race Starts In")
  (Variables|/Game/UI_test/StartCountdownUI.StartCountdownUI_C|SetMenu%20visiblity _startcountdownuiref "Visible")
  (Utilities|FlowControl|Delay 1.0)
  (Variables|/Game/UI_test/StartCountdownUI.StartCountdownUI_C|SetReady_text _startcountdownuiref "2")
  (Utilities|FlowControl|Delay 1.0)
  (Variables|/Game/UI_test/StartCountdownUI.StartCountdownUI_C|SetReady_text _startcountdownuiref "1")
  (Utilities|FlowControl|Delay 1.0)
  (Variables|/Game/UI_test/StartCountdownUI.StartCountdownUI_C|SetMenu%20visiblity _startcountdownuiref "Hidden")
  (Game|SetGamePaused false))

(event Collision|EventActorBeginOverlap
  (params (OtherActor :type Actor%20Object%20Reference)))

(event EventBeginPlay
  ;[1 1 1] Variable initialisation
  (Utilities|FlowControl|Delay 1.0)
  (bind _asplayer_controller (Utilities|Casting|CastToPlayerController (Pawn|GetController)))
  (bind _returnvalue (UserInterface|CreateWidget "/Game/Minimap/Minimap_wb.Minimap_wb_C" _asplayer_controller))
  (Variables|/Game/Minimap/Minimap_wb.Minimap_wb_C|SetMinimap_team_owner _returnvalue (Variables|Default|GetPlayer_team))
  (Variables|Default|SetMinimap_ref _returnvalue)
  (UserInterface|Viewport|AddtoPlayerScreen _returnvalue)
  (bind _returnvalue_2 (UserInterface|CreateWidget "/Game/Tesla_import/Charge_widget.Charge_widget_C" _asplayer_controller))
  (bind _output_get (Variables|Default|SetWidget_ref _returnvalue_2))
  (UserInterface|Viewport|AddtoPlayerScreen _output_get)
  (bind _returnvalue_3 (UserInterface|CreateWidget "/Game/UI_test/SampleUI.SampleUI_C" _asplayer_controller))
  (bind _output_get_2 (Variables|Default|SetSampleUI_ref _returnvalue_3))
  (UserInterface|Viewport|AddtoPlayerScreen _output_get_2)
  (Variables|/Game/Tesla_import/Charge_widget.Charge_widget_C|SetMax_energy (Variables|Default|GetWidget_ref) (Variables|Default|GetEnergy_Max))
  (Variables|/Game/Tesla_import/Charge_widget.Charge_widget_C|SetMin_energy (Variables|Default|GetWidget_ref) (Variables|Default|GetEnergy_Min))
  (bind _returnvalue_4 (UserInterface|CreateWidget "/Game/UI_test/DriverChangeUI.DriverChangeUI_C" _asplayer_controller))
  (bind _output_get_3 (Variables|Default|SetDriverChangeUI_ref _returnvalue_4))
  (UserInterface|Viewport|AddtoPlayerScreen _output_get_3)
  (bind _returnvalue_5 (UserInterface|CreateWidget "/Game/UI_test/ActivityChangeUI.ActivityChangeUI_C" _asplayer_controller))
  (bind _output_get_4 (Variables|Default|SetActivityChangeUI_ref _returnvalue_5))
  (UserInterface|Viewport|AddtoPlayerScreen _output_get_4)
  (bind _returnvalue_6 (UserInterface|CreateWidget "/Game/UI_test/StartCountdownUI.StartCountdownUI_C" _asplayer_controller))
  (bind _output_get_5 (Variables|Default|SetStartCountdownUIRef _returnvalue_6))
  (UserInterface|Viewport|AddtoPlayerScreen _output_get_5)
  (bind _asmy_game_instance (Utilities|Casting|CastToMyGameInstance (Game|GetGameInstance)))
  (Variables|Default|SetAs%20My%20Game%20Instance _asmy_game_instance)
  (Game|SetGamePaused true)
  (Variables|Default|SetEnergy_Timeout_Time (Variables|/Game/MainMenu/MyGameInstance.MyGameInstance_C|GetTimeout_time_energy (Variables|Default|GetAs%20My%20Game%20Instance))))

(event EventTick
  (params (DeltaSeconds :type Float%20%28single-precision%29))
  (bind _widget_ref (Variables|Default|GetWidget_ref))
  (bind _widget_ref_2 (Variables|Default|GetWidget_ref))
  (if (and (Utilities|IsValid (Variables|Default|GetSampleUI_ref)) (Utilities|IsValid (Variables|Default|GetWidget_ref)))
    (Utilities|FlowControl|Sequence
      (:then_0
        ;[1 1 1] Audio
        (Audio|Parameter|SetFloatParameter (Variables|Default|GetTesla%20Sound) "RPM" (Math|Float|Absolute(Float) (Class|WheeledVehicleMovementComponent|GetForwardSpeed (Variables|Default|GetVehicleMovement))) :!class /Script/Engine.AudioComponent))
      (:then_1
        ;[1 1 1] Recharge control
        (if (Variables|Default|GetPowerBool)
          (if (Variables|Default|GetEnergyInput)
            (if (< (+ (Variables|Default|GetEnergy) (Variables|Default|GetEnergyAdded)) (Variables|Default|GetEnergy_Max))
              (Variables|Default|SetEnergy (+ (Variables|Default|GetEnergy) (Variables|Default|GetEnergyAdded)))
              (else
                (bind _output_get (Variables|Default|SetEnergy (Variables|Default|GetEnergy_Max)))))
            (Variables|/Game/Tesla_import/Charge_widget.Charge_widget_C|SetEnergy_current _widget_ref _output_get)
            (Variables|Default|SetEnergyInput false)
            (Variables|Default|SetEnergyTimeout true)
            (Utilities|Time|SetTimerbyEvent (delegate Custom|EnergyTimeoutEvent) (Variables|Default|GetEnergy_Timeout_Time))
            (elif (not (< (- (Variables|Default|GetEnergy) (+ (* DeltaSeconds (Math|Float|Absolute(Float) (Input|AxisValues|GetMoveForward))) (* DeltaSeconds (Variables|Default|GetIdle_Energy_Drain)))) (Variables|Default|GetEnergy_Min)))
              (if (Variables|Default|GetGameStart)
                (Variables|Default|SetEnergy (- (Variables|Default|GetEnergy) (+ (* DeltaSeconds (Math|Float|Absolute(Float) (Input|AxisValues|GetMoveForward))) (* DeltaSeconds (Variables|Default|GetIdle_Energy_Drain))))))
              (Variables|/Game/Tesla_import/Charge_widget.Charge_widget_C|SetEnergy_current _widget_ref (Variables|Default|GetEnergy))))))
      (:then_2
        ;[1 1 1] Respawn Check and checkpoint number and answer update
        (Variables|/Game/Tesla_import/Charge_widget.Charge_widget_C|SetCheckpointsCleared (Variables|Default|GetWidget_ref) (Variables|Default|GetCheckpointsClearedNum))
        (switch int (Variables|Default|GetAnswer_num)
          (:Default
            (Variables|/Game/Tesla_import/Charge_widget.Charge_widget_C|SetAns_string _widget_ref_2 "None"))
          (:0
            (Variables|/Game/Tesla_import/Charge_widget.Charge_widget_C|SetAns_string _widget_ref_2 "(A)"))
          (:1
            (Variables|/Game/Tesla_import/Charge_widget.Charge_widget_C|SetAns_string _widget_ref_2 "(B)"))
          (:2
            (Variables|/Game/Tesla_import/Charge_widget.Charge_widget_C|SetAns_string _widget_ref_2 "(C)"))
          (:3
            (Variables|/Game/Tesla_import/Charge_widget.Charge_widget_C|SetAns_string _widget_ref_2 "Correct"))
          (:4
            (Variables|/Game/Tesla_import/Charge_widget.Charge_widget_C|SetAns_string _widget_ref_2 "Incorrect")))
        (if (Variables|Default|GetRespawnBool)
          (CallFunction|RespawnEventEvent)
          (Variables|Default|SetRespawnBool false)))
      (:then_3
        ;[1 1 1] Game over handling
        (if (Variables|/Game/MainMenu/MyGameInstance.MyGameInstance_C|GetGameOverBool (Variables|Default|GetAs%20My%20Game%20Instance))
          (if (not (Variables|Default|GetGameOver))
            (Variables|Default|SetGameOver true)
            (CallFunction|GameOverGenEvent))))
      (:then_4
        (if (Variables|/Game/MainMenu/MyGameInstance.MyGameInstance_C|GetGameStartBool (Variables|Default|GetAs%20My%20Game%20Instance))
          (if (not (Variables|Default|GetGameStart))
            (Variables|Default|SetGameStart true)
            (CallFunction|StartRaceEvent)))))))

(event Input|ActionEvents|InputActionHandbrake
  (params (Key :type Key%20Structure :default "None"))
  (bind _vehiclemovement (Variables|Default|GetVehicleMovement))
  ;[1 1 1] Movement
  (:Pressed
    (Class|WheeledVehicleMovementComponent|SetHandbrakeInput _vehiclemovement true))
  (:Released
    (Class|WheeledVehicleMovementComponent|SetHandbrakeInput _vehiclemovement false)))

(event Input|ActionEvents|InputActionHandbrake
  (params (Key :type Key%20Structure :default "None"))
  (bind _vehiclemovement (Variables|Default|GetVehicleMovement))
  ;[1 1 1] Movement
  (:Pressed
    (Class|WheeledVehicleMovementComponent|SetHandbrakeInput _vehiclemovement true))
  (:Released
    (Class|WheeledVehicleMovementComponent|SetHandbrakeInput _vehiclemovement false)))

(event Input|ActionEvents|InputActionRecharge
  (params (Key :type Key%20Structure :default "None"))
  (bind _sampleui_ref (Variables|Default|GetSampleUI_ref))
  ;[1 1 1] Recharge control
  (:Pressed
    (if (not (Variables|Default|GetPowerBool))
      (Variables|Default|SetPowerBool true)
      (Variables|Default|SetEnergy (Variables|Default|GetEnergy_Max))
      (UserInterface|Animation|PlayAnimation _sampleui_ref (Variables|/Game/UI_test/SampleUI.SampleUI_C|GetFadeOut _sampleui_ref) 0.0 1 "Forward" 1.0 false))))

(event Input|ActionEvents|InputActionRespawn
  (params (Key :type Key%20Structure :default "None"))
  ;[1 1 1] Respawn
)

(event Input|ActionEvents|InputActionGameStop
  (params (Key :type Key%20Structure :default "None"))
  ;[1 1 1] Game over handling
  (:Pressed
    (Variables|/Game/MainMenu/MyGameInstance.MyGameInstance_C|SetGameOverBool (Variables|Default|GetAs%20My%20Game%20Instance) true)
    (CallFunction|GameOverGenEvent)))

(event Input|ActionEvents|InputActionGamePlay
  (params (Key :type Key%20Structure :default "None"))
  (bind _as_my_game_instance (Variables|Default|GetAs%20My%20Game%20Instance))
  (:Pressed
    (if (Variables|/Game/MainMenu/MyGameInstance.MyGameInstance_C|GetQuestionsDone _as_my_game_instance)
      (Variables|/Game/MainMenu/MyGameInstance.MyGameInstance_C|SetGameStartBool _as_my_game_instance true)
      (CallFunction|StartRaceEvent)
      (Utilities|FlowControl|Delay 4.0))))

(event Input|AxisEvents|InputAxisMoveForward
  (params (AxisValue :type Float%20%28single-precision%29))
  ;[1 1 1] Movement
  (Class|WheeledVehicleMovementComponent|SetThrottleInput (Variables|Default|GetVehicleMovement) (* AxisValue (/ (Variables|Default|GetEnergy) (Variables|Default|GetEnergy_Max)))))

(event Input|AxisEvents|InputAxisMoveRight
  (params (AxisValue :type Float%20%28single-precision%29))
  ;[1 1 1] Movement
  (Class|WheeledVehicleMovementComponent|SetSteeringInput (Variables|Default|GetVehicleMovement) AxisValue))

(event Input|AxisEvents|InputAxisLookRight
  (params (AxisValue :type Float%20%28single-precision%29))
  ;[1 1 1] Camera
  (Transformation|AddRelativeRotation (Variables|Default|GetSpringArm) (Math|Rotator|MakeRotator 0.0 0.0 AxisValue) false false))

(event Input|AxisEvents|InputAxisLookUp
  (params (AxisValue :type Float%20%28single-precision%29))
  ;[1 1 1] Camera
  (Transformation|AddRelativeRotation (Variables|Default|GetSpringArm) (Math|Rotator|MakeRotator 0.0 AxisValue 0.0) false false))

(fn ConstructionScript)